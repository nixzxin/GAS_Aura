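; BP_FlamePillar is a flame pillar actor that animates the brightness of its FireLight to vary over time.
; From BeginPlay, it plays a flame intensity timeline whose curve scales BaseIntensity on each update, then chooses again when finished, looping continuously.
; The chooser is built to pick randomly between two timelines, but its random range is fixed at zero, so only the first is selected.
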(event `ChooseTimeline`
  (switch `int` (`KismetMathLibrary.RandomIntegerInRange` 0)
    (:`Default`
      (`self.StartTimeline_2` :!label _label))
    (:`0`
      (`self.StartTimeline_1`))
    (:`1`
      (goto _label))))

(event `self.ReceiveBeginPlay`
  (`self.ChooseTimeline`))

(event `StartTimeline_1`
  (bind (_direction _flameintensity) (`Timeline|FlameIntensityTimeLine_1` :!via `PlayFromStart`)
    (:`Update`
      (`self.ScaleFlameIntensity` _flameintensity))
    (:`Finished`
      (`self.ChooseTimeline`))))

(event `StartTimeline_2`
  (bind (_direction _flameintensitytrack) (`Timeline|FlameIntensityTimeLine_2` :!via `PlayFromStart`)
    (:`Update`
      (`self.ScaleFlameIntensity` _flameintensitytrack))
    (:`Finished`
      (`self.ChooseTimeline`))))

(fn `ScaleFlameIntensity`
  (params (Intensity :type "Float (double-precision)"))
  (`LightComponent.SetIntensity` (`self.FireLight`) (* Intensity (`self.BaseIntensity`))))

(fn `UserConstructionScript`)